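; BP_PPCharacter is a character Blueprint whose event graph holds debug and test logic.
; Pressing F runs a Visibility box trace at the actor's location and rotation with timed debug drawing, but the hit result is unused.
; Each tick, while the attribute component is valid, it prints the movement component's max speed.
; A stamina readout is left unconnected, and the construction script is empty.
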(event EventBeginPlay)

(event Collision|EventActorBeginOverlap
  (params (OtherActor :type Actor%20Object%20Reference)))

(event EventTick
  (params (DeltaSeconds :type Float%20%28single-precision%29))
  (bind _attributecomponent (Variables|Default|GetAttributeComponent)
    (:then
      (Development|PrintString (Utilities|String|ToString(Float) (Class|MovementComponent|GetMaxSpeed (Variables|Default|GetCharacterMovementComponent))) true true "(R=0.000000,G=0.660000,B=1.000000,A=1.000000)" 0.0))
    (:else)))

(event Input|KeyboardEvents|F
  (params (Key :type Key%20Structure :default "None"))
  (:Pressed
    (Collision|BoxTraceByChannel (Transformation|GetActorLocation) "0, 0, 0" "0, 0, 0" (Transformation|GetActorRotation) "TraceTypeQuery1" false 0 "ForDuration")))

(fn ConstructionScript)